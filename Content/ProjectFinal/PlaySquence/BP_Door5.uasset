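; BP_Door5 is a sliding door actor that opens through a trigger volume, either automatically or on pressing F while inside it.
; A timeline lerps the door's relative X position and reverses to close, with a sound each way.
; Flags control key-press mode, whether it can open and whether it stays open, while a Gate and FlipFlop handle key toggling.
; The construction script creates a dynamic material for configurable emissive color, saturation and power.
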(event `Key|F`
  (params (Key :type "Key Structure"))
  (bind _doorsound (`self.Doorsound`))
  (bind _returnvalue (`SceneComponent.K2_GetComponentLocation` (`self.Door_5`)))
  (:`Pressed`
    (`/Engine/EditorBlueprintResources/StandardMacros.Gate` true :!label _label
      (:`Exit`
        (`/Engine/EditorBlueprintResources/StandardMacros.FlipFlop`
          (:`A`
            (if (`self.KeepOpen`)
              (`/Engine/EditorBlueprintResources/StandardMacros.DoOnce` false
                (:`Completed`
                  _)))
            (if (`self.CanDoorOpen？`) :!label _label_2
              (`TimelineComponent.SetPlayRate` (`self.Timeline_0`) (`self.Animation Speed`))
              (`GameplayStatics.PlaySoundAtLocation` _doorsound _returnvalue (struct) 1.0 1.0 0.0 null null null)
              (bind (_direction _openclose) (`Timeline|Timeline_0` :!label _label_3)
                (:`Update`
                  (`SceneComponent.K2_SetRelativeLocation` (`self.Door_5`) (`KismetMathLibrary.MakeVector` (`KismetMathLibrary.Lerp` (`self.Door5_Closed`) (`self.Door5_Open`) _openclose)) false false)))))
          (:`B`
            (if (not (`self.KeepOpen`))
              (`GameplayStatics.PlaySoundAtLocation` _doorsound _returnvalue (struct) 1.0 1.0 0.0 null null null :!label _label_4)
              (goto _label_3 :!via `Reverse`))))))))

(event `self.Trigger.OnComponentBeginOverlap`
  (params (OverlappedComponent :type "PrimitiveComponent Object Reference") (OtherActor :type "Actor Object Reference") (OtherComp :type "PrimitiveComponent Object Reference") (OtherBodyIndex :type Integer) (bFromSweep :type Boolean) (SweepResult :type "HitResult Structure (by ref)"))
  (if (not (`self.KeepOpen`))
    (`PrimitiveComponent.SetCollisionEnabled` (`self.Door_5`) "QueryOnly"))
  (if (`self.KeyPress`)
    (`self.EnableInput` (`GameplayStatics.GetPlayerController` 0))
    (goto _label :!via `Open`)
    (else
      (goto _label_2))))

(event `self.Trigger.OnComponentEndOverlap`
  (params (OverlappedComponent :type "PrimitiveComponent Object Reference") (OtherActor :type "Actor Object Reference") (OtherComp :type "PrimitiveComponent Object Reference") (OtherBodyIndex :type Integer))
  (if (`self.CanDoorOpen？`)
    (if (`self.KeepOpen`)
      (`PrimitiveComponent.SetCollisionEnabled` (`self.Trigger`) "NoCollision")
      (elif (`self.KeyPress`)
        (goto _label :!via `Close`)
        (else
          (goto _label_4))))))

(fn `UserConstructionScript`
  (bind _returnvalue (`PrimitiveComponent.CreateDynamicMaterialInstance` (`self.Dorr5_Body`) 0 "/Game/Asset/ScFi_Doors/worn/Door5/Mat_Door5_W_Inst.Mat_Door5_W_Inst" "None"))
  (bind _output_get (set `self.MaterialReference` _returnvalue))
  (`MaterialInstanceDynamic.SetVectorParameterValue` _output_get "Emissive color" (`self.Emissive color`))
  (`MaterialInstanceDynamic.SetScalarParameterValue` _output_get "Emissive saturation" (`self.Emissive saturation`))
  (`MaterialInstanceDynamic.SetScalarParameterValue` _output_get "Emissive power" (`self.Emissive power`)))
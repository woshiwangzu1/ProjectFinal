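; Component that recomputes the state of the laser puzzle in the level, running its update once at BeginPlay.
; UpdateLazers clears IsHit on every laser receiver and reflector, then has every laser shooter cast its beam.
; It then passes each receiver's hit state to its linked actor through the BPI_React interface, if that actor implements it.
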(event `self.ReceiveBeginPlay`
  (`self.UpdateLazers`))

(fn `UpdateLazers`
  (bind _outactors (`GameplayStatics.GetAllActorsOfClass` "/Game/ProjectFinal/PlaySquence/Interactable/BPA_LazerRecevier.BPA_LazerRecevier_C"))
  (for _array_element _outactors
    (set `/Game/ProjectFinal/PlaySquence/Interactable/BPA_LazerRecevier.IsHit` false _array_element))
  (bind _outactors_2 (`GameplayStatics.GetAllActorsOfClass` "/Game/ProjectFinal/PlaySquence/Interactable/BPA_LazerReflector.BPA_LazerReflector_C"))
  (for _array_element_2 _outactors_2
    (set `/Game/ProjectFinal/PlaySquence/Interactable/BPA_LazerReflector.IsHit` false _array_element_2))
  (bind _outactors_3 (`GameplayStatics.GetAllActorsOfClass` "/Game/ProjectFinal/PlaySquence/Interactable/BPA_LazerShooter.BPA_LazerShooter_C"))
  (for _array_element_3 _outactors_3
    (`/Game/ProjectFinal/PlaySquence/Interactable/BPA_LazerShooter.CastLazer` _array_element_3))
  (bind _outactors_4 (`GameplayStatics.GetAllActorsOfClass` "/Game/ProjectFinal/PlaySquence/Interactable/BPA_LazerRecevier.BPA_LazerRecevier_C"))
  (for _array_element_4 _outactors_4
    (bind _linkedactor (`/Game/ProjectFinal/PlaySquence/Interactable/BPA_LazerRecevier.LinkedActor` _array_element_4))
    (if (`KismetSystemLibrary.DoesImplementInterface` _linkedactor "/Game/ProjectFinal/PlaySquence/Interactable/BPI_React.BPI_React_C")
      (message `/Game/ProjectFinal/PlaySquence/Interactable/BPI_React.SetState` _linkedactor (`/Game/ProjectFinal/PlaySquence/Interactable/BPA_LazerRecevier.IsHit` _array_element_4)))))